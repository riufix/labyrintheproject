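; BP_HighGravity is a box trigger volume that changes the first-person character's gravity while inside it.
; Overlap begin applies the configured GravityScale to character movement; overlap end resets it to normal.
; On entry, if the LowGravity component is not already playing, it plays it and shows the W_HighGravity widget with its down animation.
; The widget is created hidden at BeginPlay and hidden again on exit.
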(event OnComponentBeginOverlap(Box)
  (params (OverlappedComponent :type Primitive%20Component%20Object%20Reference) (OtherActor :type Actor%20Object%20Reference) (OtherComp :type Primitive%20Component%20Object%20Reference) (OtherBodyIndex :type Integer) (bFromSweep :type Boolean) (SweepResult :type Hit%20Result%20Structure%20%28by%20ref%29))
  (bind _bp_character (Variables|Default|GetBP_Character))
  (bind _low_gravity (Variables|Default|Getlow_gravity))
  (bind _highgravwidget (Variables|Default|GetHighGravWidget))
  (if (== OtherActor _bp_character)
    (Variables|/Script/Engine.CharacterMovementComponent|SetGravityScale (Variables|/Script/Engine.Character|GetCharacterMovement _bp_character) (Variables|Default|GetGravityScale))
    (if (not (Audio|Components|Audio|IsPlaying _low_gravity))
      (Audio|Components|Audio|Play _low_gravity 0.0)
      (Variables|/Script/UMG.Widget|SetVisibility _highgravwidget "Visible")
      (Default|PlayDownAnim _highgravwidget))))

(event OnComponentEndOverlap(Box)
  (params (OverlappedComponent :type Primitive%20Component%20Object%20Reference) (OtherActor :type Actor%20Object%20Reference) (OtherComp :type Primitive%20Component%20Object%20Reference) (OtherBodyIndex :type Integer))
  (bind _bp_character (Variables|Default|GetBP_Character))
  (if (== OtherActor _bp_character)
    (Variables|/Script/Engine.CharacterMovementComponent|SetGravityScale (Variables|/Script/Engine.Character|GetCharacterMovement _bp_character) 1.0)
    (Variables|/Script/UMG.Widget|SetVisibility (Variables|Default|GetHighGravWidget) "Hidden")))

(event EventBeginPlay
  (bind _asbp_first_person_character (Utilities|Casting|CastToBP_FirstPersonCharacter (Game|GetPlayerCharacter 0)))
  (Variables|Default|SetBP_Character _asbp_first_person_character)
  (bind _returnvalue (UserInterface|CreateWidget "/Game/GP/Widgets/HUD/W_HighGravity.W_HighGravity_C"))
  (bind _output_get (Variables|Default|SetHighGravWidget _returnvalue))
  (UserInterface|Viewport|AddtoViewport _output_get 0)
  (Variables|/Script/UMG.Widget|SetVisibility _output_get "Hidden"))

(fn ConstructionScript)