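; BP_InversionGravity is an actor that flips a gravity room by rotating the room itself.
; CE_InvertRoom line-traces from its Box to find a BP_GravityRoom, makes the first-person character jump, then sets it to Flying after a short delay.
; A Rotation timeline drives the room's pitch, playing forward or reversing according to IsTurned.
; On finish, the character returns to Walking and IsTurned toggles.
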(event Custom|CE_InvertRoom
  (bind _box (Variables|Default|GetBox))
  (bind _perso (Variables|Default|GetPerso))
  (bind _outhit (Collision|LineTraceByChannel (Transformation|GetWorldLocation _box) (* (Math|Vector|GetUpVector _box) "0.000000,0.000000,-10000.000000") "TraceTypeQuery1" false 0 "ForDuration"))
  (bind _asbp_gravity_room (Utilities|Casting|CastToBP_GravityRoom (.HitActor (Collision|BreakHitResult _outhit))))
  (Variables|Default|SetBP_GravityRoom _asbp_gravity_room)
  (Character|Jump _perso)
  (Utilities|FlowControl|Delay 0.2)
  (Pawn|Components|CharacterMovement|SetMovementMode (Variables|/Script/Engine.Character|GetCharacterMovement _perso) "MOVE_Flying" 0)
  (if (Variables|Default|GetisTurned)
    (bind _rotationfloat (Timeline|Rotation ReverseFromEnd)
      (:Update
        (Transformation|SetActorRotation (Variables|Default|GetBP_GravityRoom) (Math|Rotator|MakeRotator 0.0 _rotationfloat 0.0)))
      (:Finished
        (Pawn|Components|CharacterMovement|SetMovementMode (Variables|/Script/Engine.Character|GetCharacterMovement (Variables|Default|GetPerso)) "MOVE_Walking" 0)
        (if (Variables|Default|GetisTurned)
          (Variables|Default|SetisTurned false)
          (else
            (Variables|Default|SetisTurned true)))))
    (else
      (Timeline|Rotation Play))))

(event EventBeginPlay
  (bind _asbp_first_person_character (Utilities|Casting|CastToBP_FirstPersonCharacter (Game|GetPlayerCharacter 0)))
  (Variables|Default|SetPerso _asbp_first_person_character))

(fn ConstructionScript)