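; BP_Ventilateur is a fan that pushes the first-person player through its box volume while active.
; Overlapping the box switches the character to Flying at the fan's max fly speed, and leaving restores Walking.
; Tick adds movement input along the box's forward vector, scaled by X/Y values remapped from its yaw at BeginPlay.
; OnActivate stops the fan once all linked pressure plates, or levers if none, are activated.
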(event OnComponentBeginOverlap(Box)
  (params (OverlappedComponent :type Primitive%20Component%20Object%20Reference) (OtherActor :type Actor%20Object%20Reference) (OtherComp :type Primitive%20Component%20Object%20Reference) (OtherBodyIndex :type Integer) (bFromSweep :type Boolean) (SweepResult :type Hit%20Result%20Structure%20%28by%20ref%29))
  (bind _bp_character (Variables|Default|GetBP_Character))
  (bind _charactermovement (Variables|/Script/Engine.Character|GetCharacterMovement _bp_character))
  (if (== OtherActor _bp_character)
    (if (Variables|Default|GetisActivated)
      (Variables|Default|SetisInFan true)
      (Pawn|Components|CharacterMovement|SetMovementMode _charactermovement "MOVE_Flying" 0)
      (Variables|/Script/Engine.CharacterMovementComponent|SetMaxFlySpeed _charactermovement (Variables|Default|GetMaxFlySpeed)))))

(event OnComponentEndOverlap(Box)
  (params (OverlappedComponent :type Primitive%20Component%20Object%20Reference) (OtherActor :type Actor%20Object%20Reference) (OtherComp :type Primitive%20Component%20Object%20Reference) (OtherBodyIndex :type Integer))
  (bind _bp_character (Variables|Default|GetBP_Character))
  (bind _charactermovement (Variables|/Script/Engine.Character|GetCharacterMovement _bp_character))
  (if (== OtherActor _bp_character)
    (if (Variables|Default|GetisActivated)
      (Variables|Default|SetisInFan false)
      (Pawn|Components|CharacterMovement|SetMovementMode _charactermovement "MOVE_Walking" 0)
      (Variables|/Script/Engine.CharacterMovementComponent|SetMaxFlySpeed _charactermovement 2e+02))))

(event EventBeginPlay
  (bind _box (Variables|Default|GetBox))
  (bind _returnvalue (Transformation|GetWorldRotation _box))
  (bind _asbp_first_person_character (Utilities|Casting|CastToBP_FirstPersonCharacter (Game|GetPlayerCharacter 0)))
  (Variables|Default|SetBP_Character _asbp_first_person_character)
  (if (!= (.yaw _returnvalue) 0.0)
    (Variables|Default|SetX (Variables|Default|GetX)))
  (if (== (.yaw _returnvalue) 9e+01)
    (Variables|Default|SetY (Variables|Default|GetX))
    (Variables|Default|SetX 0.0)
    (elif (== (.yaw _returnvalue) -9e+01)
      (Variables|Default|SetY (Variables|Default|GetX))
      (Variables|Default|SetX 0.0))))

(event EventOnActivate
  (bind _listedeplaquedepression (Variables|Default|GetListedePlaqueDePression))
  (bind _listelevier (Variables|Default|GetListeLevier))
  (Variables|Default|SetisActivated false)
  (if (> (Utilities|Array|Length _listedeplaquedepression) 0)
    (for _array_element _listedeplaquedepression
      (if (not (Variables|/Game/Effects/BP_PlaquePression.BP_PlaquePression_C|GetisActivated _array_element))
        (Variables|Default|SetisActivated true)))
    (if (not (Variables|Default|GetisActivated)) :!label _label
      (Audio|Components|Audio|Stop (Variables|Default|Getfan) :!label _label_2))
    (elif (> (Utilities|Array|Length _listelevier) 0)
      (for _array_element_2 _listelevier
        (if (not (Variables|/Game/Effects/BP_Levier.BP_Levier_C|GetisActivated _array_element_2))
          (Variables|Default|SetisActivated true)))
      (goto _label)
      (else
        (goto _label_2)))))

(event EventTick
  (params (DeltaSeconds :type Float%20%28single-precision%29))
  (if (Variables|Default|GetisActivated)
    (if (Variables|Default|GetisInFan)
      (Pawn|Input|AddMovementInput (Variables|Default|GetBP_Character) (* (Math|Vector|GetForwardVector (Variables|Default|GetBox)) (Math|Vector|MakeVector (Variables|Default|GetX) (Variables|Default|GetY) 0.0)) 1.0 false))))

(fn ConstructionScript)