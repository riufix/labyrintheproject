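; Door actor that slides vertically open or closed when activated, gated by linked pressure plates or levers.
; OnActivate requires every listed pressure plate to be activated, checks levers only if no plates are listed, and toggles freely when both lists are empty.
; A FlipFlop alternately plays and reverses a timeline that lerps the door's relative Z to a configurable height, with a sound on finish.
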(event EventOnActivate
  (bind _listeplaquedepressionpourlouvrir (Variables|Default|GetListePlaqueDePressionPourLouvrir))
  (bind _listelevier (Variables|Default|GetListeLevier))
  (Variables|Default|SetcanOpen true)
  (if (> (Utilities|Array|Length _listeplaquedepressionpourlouvrir) 0)
    (for _array_element _listeplaquedepressionpourlouvrir
      (if (not (Variables|/Game/Effects/BP_PlaquePression.BP_PlaquePression_C|GetisActivated _array_element))
        (Variables|Default|SetcanOpen false)))
    (if (Variables|Default|GetcanOpen) :!label _label
      (Utilities|FlowControl|FlipFlop :!label _label_2
        (:A
          (bind _newtrack_0 (Timeline|CloseDoor Play)
            (:Update
              (Transformation|SetRelativeLocation (Variables|Default|GetDoor) (Math|Vector|MakeVector 0.0 0.0 (Math|Float|Lerp 0.0 (Variables|Default|GetHauteurOuverturePorte) _newtrack_0)) false false))
            (:Finished
              (Audio|PlaySound2D "/Game/SD/door_open_closed.door_open_closed" 1.0 1.0 0.0 0 0))))
        (:B
          (Timeline|CloseDoor ReverseFromEnd))))
    (elif (> (Utilities|Array|Length _listelevier) 0)
      (for _array_element_2 _listelevier
        (if (not (Variables|/Game/Effects/BP_Levier.BP_Levier_C|GetisActivated _array_element_2))
          (Variables|Default|SetcanOpen false)))
      (goto _label)
      (else
        (goto _label_2)))))

(fn ConstructionScript)