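; BP_Fire is a fire hazard that alternates between active and inactive and kills the first-person player character.
; BeginPlay caches the player character, then a looping Delay and FlipFlop toggles IsActive every few seconds.
; Box overlap events set IsInsideFire without checking which actor overlaps.
; Tick calls CEDie on the cached player whenever both flags are true.
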(event OnComponentBeginOverlap(Box)
  (params (OverlappedComponent :type Primitive%20Component%20Object%20Reference) (OtherActor :type Actor%20Object%20Reference) (OtherComp :type Primitive%20Component%20Object%20Reference) (OtherBodyIndex :type Integer) (bFromSweep :type Boolean) (SweepResult :type Hit%20Result%20Structure%20%28by%20ref%29))
  (Variables|Default|SetisInsideFire true))

(event OnComponentEndOverlap(Box)
  (params (OverlappedComponent :type Primitive%20Component%20Object%20Reference) (OtherActor :type Actor%20Object%20Reference) (OtherComp :type Primitive%20Component%20Object%20Reference) (OtherBodyIndex :type Integer))
  (Variables|Default|SetisInsideFire false))

(event EventBeginPlay
  (bind _asbp_first_person_character (Utilities|Casting|CastToBP_FirstPersonCharacter (Game|GetPlayerCharacter 0)))
  (Variables|Default|SetBP_Character _asbp_first_person_character)
  (Utilities|FlowControl|Delay 3.0 :!label _label)
  (Utilities|FlowControl|FlipFlop
    (:A
      (Variables|Default|SetisActive true)
      (goto _label))
    (:B
      (Variables|Default|SetisActive false)
      (goto _label))))

(event EventTick
  (params (DeltaSeconds :type Float%20%28single-precision%29))
  (if (Variables|Default|GetisInsideFire)
    (if (Variables|Default|GetisActive)
      (Default|CEDie (Variables|Default|GetBP_Character)))))

(fn ConstructionScript)