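; BP_Levier is a one-shot lever that the player can interact with to trigger another actor.
; On the first interaction it plays a sound, sets an activated flag and rotates the lever mesh through a timeline.
; When the timeline finishes it sends an activate message to its ControlledActor.
; It always reports itself as interactible, so the flag alone blocks repeat activations.
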(event EventBeginPlay)

(event Collision|EventActorBeginOverlap
  (params (OtherActor :type Actor%20Object%20Reference)))

(event EventTick
  (params (DeltaSeconds :type Float%20%28single-precision%29)))

(event EventOnInteract
  (params (Character :type BP%20First%20Person%20Character%20Object%20Reference))
  (if (not (Variables|Default|GetisActivated))
    (Audio|PlaySound2D "/Game/SD/Jehan/levier.levier" 1.0 1.0 0.0 0 0)
    (Variables|Default|SetisActivated true)
    (bind _newtrack_0 (Timeline|TimelineLevier Play)
      (:Update
        (Transformation|SetRelativeRotation (Variables|Default|GetLever) (Math|Rotator|Lerp(Rotator) "0, 0, 0" "0.000000,0.000000,180.000000" _newtrack_0) false false))
      (:Finished
        (Class|BPIRotate|OnActivate(Message) (Variables|Default|GetControlledActor))))))

(fn ConstructionScript)

(fn IsInteractible
  (return true))