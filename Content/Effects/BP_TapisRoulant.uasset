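; BP_TapisRoulant is a conveyor belt that pushes the first-person character along while they stand in its box.
; Box overlap flags the character and overrides air control and walk speed.
; Tick adds movement input along the box's forward vector, scaled by X/Y remapped at BeginPlay for ±90° yaw, only while grounded.
; Any end overlap, without an actor check, restores cached air control and a hard-coded walk speed.
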(event OnComponentBeginOverlap(Box)
  (params (OverlappedComponent :type Primitive%20Component%20Object%20Reference) (OtherActor :type Actor%20Object%20Reference) (OtherComp :type Primitive%20Component%20Object%20Reference) (OtherBodyIndex :type Integer) (bFromSweep :type Boolean) (SweepResult :type Hit%20Result%20Structure%20%28by%20ref%29))
  (bind _bp_character (Variables|Default|GetBP_Character))
  (bind _charactermovement (Variables|/Script/Engine.Character|GetCharacterMovement _bp_character))
  (if (== OtherActor _bp_character)
    (Variables|Default|SetisInside true)
    (Variables|/Game/FirstPerson/Blueprints/BP_FirstPersonCharacter.BP_FirstPersonCharacter_C|SetisInTapisRoulant _bp_character true)
    (Variables|/Script/Engine.CharacterMovementComponent|SetAirControl _charactermovement (Variables|Default|GetAir%20Control))
    (Variables|/Script/Engine.CharacterMovementComponent|SetMaxWalkSpeed _charactermovement (Variables|Default|GetMax%20Walk%20Speed))))

(event OnComponentEndOverlap(Box)
  (params (OverlappedComponent :type Primitive%20Component%20Object%20Reference) (OtherActor :type Actor%20Object%20Reference) (OtherComp :type Primitive%20Component%20Object%20Reference) (OtherBodyIndex :type Integer))
  (bind _bp_character (Variables|Default|GetBP_Character))
  (bind _charactermovement (Variables|/Script/Engine.Character|GetCharacterMovement _bp_character))
  (Variables|Default|SetisInside false)
  (Variables|/Game/FirstPerson/Blueprints/BP_FirstPersonCharacter.BP_FirstPersonCharacter_C|SetisInTapisRoulant _bp_character false)
  (Variables|/Script/Engine.CharacterMovementComponent|SetAirControl _charactermovement (Variables|Default|GetAirControlDeBase))
  (Variables|/Script/Engine.CharacterMovementComponent|SetMaxWalkSpeed _charactermovement 4e+02))

(event EventBeginPlay
  (bind _box (Variables|Default|GetBox))
  (bind _returnvalue (Transformation|GetWorldRotation _box))
  (bind _asbp_first_person_character (Utilities|Casting|CastToBP_FirstPersonCharacter (Game|GetPlayerCharacter 0)))
  (bind _output_get (Variables|Default|SetBP_Character _asbp_first_person_character))
  (Variables|Default|SetAirControlDeBase (Variables|/Script/Engine.CharacterMovementComponent|GetAirControl (Variables|/Script/Engine.Character|GetCharacterMovement _output_get)))
  (if (!= (.yaw _returnvalue) 0.0)
    (Variables|Default|SetX (Variables|Default|GetX)))
  (if (== (.yaw _returnvalue) 9e+01)
    (Variables|Default|SetY (Variables|Default|GetX))
    (Variables|Default|SetX 0.0)
    (elif (== (.yaw _returnvalue) -9e+01)
      (Variables|Default|SetY (Variables|Default|GetX))
      (Variables|Default|SetX 0.0))))

(event EventTick
  (params (DeltaSeconds :type Float%20%28single-precision%29))
  (bind _bp_character (Variables|Default|GetBP_Character))
  (if (Variables|Default|GetisInside)
    (if (AI|Components|NavMovement|IsMovingonGround (Variables|/Script/Engine.Character|GetCharacterMovement _bp_character))
      (Pawn|Input|AddMovementInput _bp_character (* (Math|Vector|GetForwardVector (Variables|Default|GetBox)) (Math|Vector|MakeVector (Variables|Default|GetX) (Variables|Default|GetY) 0.0)) 1.0 false))))

(fn ConstructionScript)