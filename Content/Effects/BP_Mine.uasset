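; BP_Mine is a mine that kills the first-person player character when they enter one of its trigger boxes.
; Box fires on any player overlap, while BoxForCrouch fires only if the player is crouching as the overlap begins.
; Either trigger disables movement and plays an explosion sound, then after a short delay calls CEDie on the player and destroys the mine.
; The cached game mode reference is unused.
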(event OnComponentBeginOverlap(Box)
  (params (OverlappedComponent :type Primitive%20Component%20Object%20Reference) (OtherActor :type Actor%20Object%20Reference) (OtherComp :type Primitive%20Component%20Object%20Reference) (OtherBodyIndex :type Integer) (bFromSweep :type Boolean) (SweepResult :type Hit%20Result%20Structure%20%28by%20ref%29))
  (bind _bp_charc (Variables|Default|GetBP_Charc))
  (if (== OtherActor _bp_charc)
    (CallFunction|ShowDamage)
    (Utilities|FlowControl|Delay 0.3)
    (Default|CEDie _bp_charc)
    (Actor|DestroyActor)))

(event OnComponentBeginOverlap(BoxForCrouch)
  (params (OverlappedComponent :type Primitive%20Component%20Object%20Reference) (OtherActor :type Actor%20Object%20Reference) (OtherComp :type Primitive%20Component%20Object%20Reference) (OtherBodyIndex :type Integer) (bFromSweep :type Boolean) (SweepResult :type Hit%20Result%20Structure%20%28by%20ref%29))
  (bind _bp_charc (Variables|Default|GetBP_Charc))
  (if (== OtherActor _bp_charc)
    (if (AI|Components|NavMovement|IsCrouching (Variables|/Script/Engine.Character|GetCharacterMovement _bp_charc))
      (CallFunction|ShowDamage)
      (Utilities|FlowControl|Delay 0.3)
      (Default|CEDie (Variables|Default|GetBP_Charc))
      (Actor|DestroyActor))))

(event EventBeginPlay
  (bind _asbp_first_person_character (Utilities|Casting|CastToBP_FirstPersonCharacter (Game|GetPlayerCharacter 0)))
  (Variables|Default|SetBP_Charc _asbp_first_person_character)
  (bind _asbp_first_person_game_mode (Utilities|Casting|CastToBP_FirstPersonGameMode (Game|GetGameMode)))
  (Variables|Default|SetGame%20Mode _asbp_first_person_game_mode))

(fn ConstructionScript)

(fn ShowDamage
  (Pawn|Components|CharacterMovement|DisableMovement (Variables|/Script/Engine.Character|GetCharacterMovement (Variables|Default|GetBP_Charc)))
  (Audio|PlaySound2D "/Game/SD/Actors/mineExplosion_01.mineExplosion_01" 1.0 1.0 0.0 0 0) ; Son trop long
)