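; BP_LowGravity is a volume effect that changes the first-person player's gravity scale and air control while inside its Box.
; BeginPlay caches player 0's character and copies the volume's own AirControl into StartAirControl.
; Overlap begin applies the configured values to that character's movement component.
; Overlap end resets gravity scale to default and applies StartAirControl, which holds the volume's value rather than the character's original.
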(event OnComponentBeginOverlap(Box)
  (params (OverlappedComponent :type Primitive%20Component%20Object%20Reference) (OtherActor :type Actor%20Object%20Reference) (OtherComp :type Primitive%20Component%20Object%20Reference) (OtherBodyIndex :type Integer) (bFromSweep :type Boolean) (SweepResult :type Hit%20Result%20Structure%20%28by%20ref%29))
  (bind _bp_character (Variables|Default|GetBP_Character))
  (bind _charactermovement (Variables|/Script/Engine.Character|GetCharacterMovement _bp_character))
  (if (== OtherActor _bp_character)
    (Variables|/Script/Engine.CharacterMovementComponent|SetGravityScale _charactermovement (Variables|Default|GetGravityScale))
    (Variables|/Script/Engine.CharacterMovementComponent|SetAirControl _charactermovement (Variables|Default|GetAir%20Control))))

(event OnComponentEndOverlap(Box)
  (params (OverlappedComponent :type Primitive%20Component%20Object%20Reference) (OtherActor :type Actor%20Object%20Reference) (OtherComp :type Primitive%20Component%20Object%20Reference) (OtherBodyIndex :type Integer))
  (bind _bp_character (Variables|Default|GetBP_Character))
  (bind _charactermovement (Variables|/Script/Engine.Character|GetCharacterMovement _bp_character))
  (if (== OtherActor _bp_character)
    (Variables|/Script/Engine.CharacterMovementComponent|SetGravityScale _charactermovement 1.0)
    (Variables|/Script/Engine.CharacterMovementComponent|SetAirControl _charactermovement (Variables|Default|GetStartAirControl))))

(event EventBeginPlay
  (bind _asbp_first_person_character (Utilities|Casting|CastToBP_FirstPersonCharacter (Game|GetPlayerCharacter 0)))
  (Variables|Default|SetBP_Character _asbp_first_person_character)
  (Variables|Default|SetStartAirControl (Variables|Default|GetAir%20Control)))

(fn ConstructionScript)