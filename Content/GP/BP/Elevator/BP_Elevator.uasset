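; BP_Elevator is an elevator actor that streams in a floor when the first-person player steps inside.
; On BeginPlay it caches the BP_FirstPersonCharacter reference.
; Overlap of its Box by that character sets IsIn, waits WaitBeforeLoading, then loads FloorToLoad as a level instance.
; IsIn is never reset, and IsInteractible always returns false.
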(event OnComponentBeginOverlap(Box)
  (params (OverlappedComponent :type Primitive%20Component%20Object%20Reference) (OtherActor :type Actor%20Object%20Reference) (OtherComp :type Primitive%20Component%20Object%20Reference) (OtherBodyIndex :type Integer) (bFromSweep :type Boolean) (SweepResult :type Hit%20Result%20Structure%20%28by%20ref%29))
  (if (== OtherActor (Variables|Default|GetFirst%20Person%20Chara))
    (bind _output_get (Variables|Default|SetIs%20In? true))
    (if _output_get
      (Utilities|FlowControl|Delay (Variables|Default|GetWait%20Before%20Loading))
      (Class|LevelStreamingDynamic|LoadLevelInstancebySoftObjectPtr (Variables|Default|GetFloor%20To%20Load) "0, 0, 0" "0, 0, 0" "" 0 false))))

(event EventBeginPlay
  (bind _asbp_first_person_character (Utilities|Casting|CastToBP_FirstPersonCharacter (Game|GetPlayerCharacter 0)))
  (Variables|Default|SetFirst%20Person%20Chara _asbp_first_person_character))

(fn ConstructionScript)

(fn IsInteractible
  (return false))