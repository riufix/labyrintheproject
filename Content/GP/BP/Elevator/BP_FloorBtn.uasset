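; BP_FloorBtn is an interactable elevator floor button that loads a selected level as a level instance.
; On BeginPlay it caches the player's BP_FirstPersonCharacter.
; On interact it loads LevelSelected by soft object pointer and prints a debug message, but only while the character's HasPressedButton flag is false.
; It only reads that flag and never sets it, and it always reports itself as interactible.
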(event EventBeginPlay
  (bind _asbp_first_person_character (Utilities|Casting|CastToBP_FirstPersonCharacter (Game|GetPlayerCharacter 0)))
  (Variables|Default|SetFirst%20Person%20Chara _asbp_first_person_character))

(event EventOnInteract
  (params (Character :type BP%20First%20Person%20Character%20Object%20Reference))
  (if (not (Variables|/Game/FirstPerson/Blueprints/BP_FirstPersonCharacter.BP_FirstPersonCharacter_C|GethasPressedButton (Variables|Default|GetFirst%20Person%20Chara)))
    (Class|LevelStreamingDynamic|LoadLevelInstancebySoftObjectPtr (Variables|Default|GetLevel%20Selected) "0, 0, 0" "0, 0, 0" "" 0 false)
    (Development|PrintString "load")))

(fn ConstructionScript)

(fn IsInteractible
  (return true))