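; BP_circularSaw is a saw hazard that kills the first-person player on contact.
; On BeginPlay it caches the player character, and a hit on the Saw component by that character calls its CEDie event.
; A timeline-driven back-and-forth movement between the saw's start position and a Destination offset is present but disconnected, so it never runs.
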(event OnComponentHit(saw)
  (params (HitComponent :type Primitive%20Component%20Object%20Reference) (OtherActor :type Actor%20Object%20Reference) (OtherComp :type Primitive%20Component%20Object%20Reference) (NormalImpulse :type Vector :default "0, 0, 0") (Hit :type Hit%20Result%20Structure%20%28by%20ref%29))
  (bind _player (Variables|Default|GetPlayer))
  (if (== OtherActor _player)
    (Default|CEDie _player)))

(event EventBeginPlay
  (bind _asbp_first_person_character (Utilities|Casting|CastToBP_FirstPersonCharacter (Game|GetPlayerCharacter 0)))
  (Variables|Default|SetPlayer _asbp_first_person_character))

(fn ConstructionScript)