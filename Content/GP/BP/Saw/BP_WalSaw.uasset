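; BP_WalSaw is a saw trap on a swinging arm that kills the first-person player on contact.
; Tick waits TimeToStart before playing the UpDown timeline, which yaws the Arm toward AngleToOsciliate and reverses when finished, so it oscillates.
; A saw hit on the cached player disables movement, shows the GameMode's PiquesHUD and plays a stab sound.
; After a short delay it hides the HUD and calls CEDie on the player.
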(event OnComponentHit(Saw)
  (params (HitComponent :type Primitive%20Component%20Object%20Reference) (OtherActor :type Actor%20Object%20Reference) (OtherComp :type Primitive%20Component%20Object%20Reference) (NormalImpulse :type Vector :default "0, 0, 0") (Hit :type Hit%20Result%20Structure%20%28by%20ref%29))
  (bind _first_person_chara (Variables|Default|GetFirst%20Person%20Chara))
  (if (== OtherActor _first_person_chara)
    (CallFunction|ShowDamage)
    (Utilities|FlowControl|Delay 1.0)
    (Widget|SetVisibility (Variables|/Game/FirstPerson/Blueprints/BP_FirstPersonGameMode.BP_FirstPersonGameMode_C|GetPiquesHUD (Variables|Default|GetGame%20mode)) "Hidden")
    (Default|CEDie _first_person_chara)))

(event Custom|Reverse
  (bind _up_down_movement (Timeline|Up/Down Reverse)
    (:Update
      (Transformation|SetRelativeRotation (Variables|Default|GetArm) (Math|Rotator|MakeRotator 0.0 0.0 (Math|Float|Lerp 0.0 (Variables|Default|GetAngle%20To%20Osciliate) _up_down_movement)) false false))
    (:Finished
      (CallFunction|Reverse))))

(event EventBeginPlay
  (bind _asbp_first_person_character (Utilities|Casting|CastToBP_FirstPersonCharacter (Game|GetPlayerCharacter 0)))
  (Variables|Default|SetFirst%20Person%20Chara _asbp_first_person_character))

(event EventTick
  (params (DeltaSeconds :type Float%20%28single-precision%29))
  (Utilities|FlowControl|Delay (Variables|Default|GetTime%20To%20Start))
  (bind _up_down_movement (Timeline|Up/Down Play)
    (:Update
      (Transformation|SetRelativeRotation (Variables|Default|GetArm) (Math|Rotator|MakeRotator 0.0 0.0 (Math|Float|Lerp 0.0 (Variables|Default|GetAngle%20To%20Osciliate) _up_down_movement)) false false))
    (:Finished
      (CallFunction|Reverse))))

(fn ConstructionScript)

(fn ShowDamage
  (Pawn|Components|CharacterMovement|DisableMovement (Variables|/Script/Engine.Character|GetCharacterMovement (Variables|Default|GetFirst%20Person%20Chara)))
  (Variables|/Script/UMG.Widget|SetVisibility (Variables|/Game/FirstPerson/Blueprints/BP_FirstPersonGameMode.BP_FirstPersonGameMode_C|GetPiquesHUD (Variables|Default|GetGame%20mode)) "Visible")
  (Audio|PlaySound2D "/Game/SD/Actors/piquesStab.piquesStab" 1.0 1.0 0.0 0 0) ; Son trop long
)