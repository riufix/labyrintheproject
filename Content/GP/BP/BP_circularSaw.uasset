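; BP_circularSaw is a circular saw actor that slides back and forth along a short straight path.
; BeginPlay takes the saw component's world position as the start and derives the end from a fixed world Y offset.
; The BackInForth timeline lerps the actor's location without sweep, and on finishing flips AtDestination to replay from start or reverse from end.
; The overlap event is empty, so contact has no effect here.
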(event EventBeginPlay
  (bind _output_get (Variables|Default|SetstartPos (Transformation|GetWorldLocation (Variables|Default|Getsaw))))
  (Variables|Default|SetendPos (+ _output_get "0.000000,100.000000,0.000000"))
  (bind _location_at_time (Timeline|BackInForth Play)
    (:Update
      (Transformation|SetActorLocation (Math|Vector|Lerp(Vector) (Variables|Default|GetstartPos) (Variables|Default|GetendPos) _location_at_time) false false))
    (:Finished
      (if (Variables|Default|GetAtDestination?)
        (Variables|Default|SetAtDestination? false)
        (Timeline|BackInForth ReverseFromEnd)
        (else
          (Variables|Default|SetAtDestination? true)
          (Timeline|BackInForth PlayFromStart))))))

(event Collision|EventActorBeginOverlap
  (params (OtherActor :type Actor%20Object%20Reference)))

(fn ConstructionScript)