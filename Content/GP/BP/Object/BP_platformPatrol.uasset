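; Moving platform actor that patrols continuously between a start point and an EndPosition.
; On BeginPlay it stores the Cube's world location as the start, then runs the Patrol timeline, whose BackInForth track lerps the actor's location without sweeping.
; When the timeline finishes, the AtDestination flag toggles and selects playing from the start or reversing from the end, keeping the motion looping.
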(event EventBeginPlay
  (Variables|Default|SetStart%20position (Transformation|GetWorldLocation (Variables|Default|GetCube)))
  (bind _back__in_forth (Timeline|Patrol Play)
    (:Update
      (Transformation|SetActorLocation (Math|Vector|Lerp(Vector) (Variables|Default|GetStart%20position) (Variables|Default|GetEnd%20Position) _back__in_forth) false false))
    (:Finished
      (if (Variables|Default|GetAtDestination?)
        (Variables|Default|SetAtDestination? false)
        (Timeline|Patrol ReverseFromEnd)
        (else
          (Variables|Default|SetAtDestination? true)
          (Timeline|Patrol PlayFromStart))))))

(event Collision|EventActorBeginOverlap
  (params (OtherActor :type Actor%20Object%20Reference)))

(fn ConstructionScript)