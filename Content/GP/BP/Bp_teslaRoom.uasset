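; Tesla room actor that acts as a hazard, halting the player's movement on overlap while IsEnable is true.
; BeginPlay starts a looping timer with no visible bound event, then runs a branch that reassigns IsEnable its existing value, so nothing toggles it.
; Any overlapping actor triggers StopMovement on player controller 0 and a debug print of the flag.
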(event EventBeginPlay
  (Utilities|Time|SetTimerbyEvent 0 (Variables|Default|Gettime) true)
  (if (Variables|Default|GetisEnable?)
    (Variables|Default|SetisEnable? true)
    (else
      (Variables|Default|SetisEnable? false))))

(event Collision|EventActorBeginOverlap
  (params (OtherActor :type Actor%20Object%20Reference))
  (bind _isenable_ (Variables|Default|GetisEnable?))
  (if _isenable_
    (AI|Navigation|StopMovement (Game|GetPlayerController 0))
    (Development|PrintString (Utilities|String|ToString(Boolean) _isenable_))))

(fn ConstructionScript)