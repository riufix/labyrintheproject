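; BP_Tp is a teleporter that moves the first-person player character to the location of a linked Actor when the player enters its Box.
; Each teleport sets CantGoBack on both itself and the linked Actor to block bouncing straight back.
; An overlap while the linked flag is set skips teleporting and clears both flags after a TimeBeforeTpingBack delay.
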(event OnComponentBeginOverlap(Box)
  (params (OverlappedComponent :type Primitive%20Component%20Object%20Reference) (OtherActor :type Actor%20Object%20Reference) (OtherComp :type Primitive%20Component%20Object%20Reference) (OtherBodyIndex :type Integer) (bFromSweep :type Boolean) (SweepResult :type Hit%20Result%20Structure%20%28by%20ref%29))
  (bind _actor (Variables|Default|Getactor))
  (if (== OtherActor (Variables|Default|GetFirst%20Person%20Chara))
    (if (Variables|BP_Tp_C|GetCant%20Go%20Back? _actor)
      (Utilities|FlowControl|Delay (Variables|Default|GetTime%20before%20tping%20back))
      (Variables|Default|SetCant%20Go%20Back? false)
      (Variables|BP_Tp_C|SetCant%20Go%20Back? (Variables|Default|Getactor) false)
      (else
        (Variables|Default|SetCant%20Go%20Back? true)
        (Variables|BP_Tp_C|SetCant%20Go%20Back? _actor true)
        (Transformation|SetActorRelativeLocation (Variables|Default|GetFirst%20Person%20Chara) (Transformation|GetActorLocation _actor) false true)))))

(event EventBeginPlay
  (bind _asbp_first_person_character (Utilities|Casting|CastToBP_FirstPersonCharacter (Game|GetPlayerCharacter 0)))
  (Variables|Default|SetFirst%20Person%20Chara _asbp_first_person_character))

(fn ConstructionScript)