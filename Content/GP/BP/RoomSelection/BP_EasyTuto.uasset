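; BP_EasyTuto is an interactable button in the room selection area that streams in a room level and opens a door.
; On interaction, unless the player character has already pressed a button, it loads RoomToLoad as a level instance offset from the button's cylinder.
; It sets the player's HasPressedButton flag, animates the cylinder down via a timeline, then plays a sound and, after a delay, activates the linked door (Porte).
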(event Collision|EventActorBeginOverlap
  (params (OtherActor :type Actor%20Object%20Reference)))

(event EventTick
  (params (DeltaSeconds :type Float%20%28single-precision%29)))

(event EventOnInteract
  (params (Character :type BP%20First%20Person%20Character%20Object%20Reference))
  (if (not (Variables|/Game/FirstPerson/Blueprints/BP_FirstPersonCharacter.BP_FirstPersonCharacter_C|GethasPressedButton (Variables|Default|GetAs%20BP%20First%20Person%20Character)))
    ;[1 1 1] streaming levels
    (Class|LevelStreamingDynamic|LoadLevelInstancebySoftObjectPtr (Variables|Default|GetRoom%20to%20load) (+ (Variables|Default|GetSpawnRoomPosition) (Transformation|GetWorldLocation (Variables|Default|GetCylinder))) "0, 0, 0" "" 0 false)
    (Variables|/Game/FirstPerson/Blueprints/BP_FirstPersonCharacter.BP_FirstPersonCharacter_C|SethasPressedButton (Variables|Default|GetAs%20BP%20First%20Person%20Character) true)
    (Audio|Components|Audio|Play (Variables|Default|Getpush) 0.0)
    (bind _newtrack_0 (Timeline|Timeline Play)
      (:Update
        (Transformation|SetRelativeLocation (Variables|Default|GetCylinder) (Math|Vector|MakeVector 0.0 0.0 (Math|Float|Lerp 0.0 -8.0 _newtrack_0)) false false))
      (:Finished
        (Audio|PlaySound2D "/Game/SD/Jehan/Pre_Opening_Door.Pre_Opening_Door" 1.0 1.0 0.0 0 0)
        (Utilities|FlowControl|Delay 3.0)
        (Class|BPIRotate|OnActivate(Message) (Variables|Default|GetPorte))
        (if (not (Variables|Default|GetisPressed))
          (Variables|Default|SetisPressed true))))))

(event EventBeginPlay
  (bind _asbp_first_person_character (Utilities|Casting|CastToBP_FirstPersonCharacter (Game|GetPlayerCharacter 0)))
  (Variables|Default|SetAs%20BP%20First%20Person%20Character _asbp_first_person_character))

(fn ConstructionScript)

(fn IsInteractible
  (return true))