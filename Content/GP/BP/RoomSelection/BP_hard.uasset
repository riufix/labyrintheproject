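; BP_hard is an interactible room selection actor for the hard option, always available for interaction.
; On interact, it loads RoomToLoad as a level instance at its Cylinder's world location plus the SpawnRoomPosition offset.
; It then prints a debug string and sends StaticMeshQueVousVoulezAfficher to PlaneAvecLicone through OnActivateMessage.
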(event EventBeginPlay)

(event Collision|EventActorBeginOverlap
  (params (OtherActor :type Actor%20Object%20Reference)))

(event EventTick
  (params (DeltaSeconds :type Float%20%28single-precision%29)))

(event EventOnInteract
  (params (Character :type BP%20First%20Person%20Character%20Object%20Reference))
  (Class|LevelStreamingDynamic|LoadLevelInstancebySoftObjectPtr (Variables|Default|GetRoom%20to%20load) (+ (Transformation|GetWorldLocation (Variables|Default|GetCylinder)) (Variables|Default|GetSpawnRoomPosition)) "0, 0, 0" "" 0 false)
  (Development|PrintString "Hard spawned")
  (Class|IIcone|OnActivate(Message) (Variables|Default|GetPlaneAvecLicone) (Variables|Default|GetStaticMeshQueVousVoulezAfficher)))

(fn ConstructionScript)

(fn IsInteractible
  (return true))