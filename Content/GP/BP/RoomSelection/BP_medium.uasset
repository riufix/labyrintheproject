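; BP_medium is an interactable room-selection button that, when pressed, streams in a chosen room and adds bonus time to the player's countdown.
; On interact, it loads the room level at an offset from the button, sends an icon and bonus to a display plane, and updates the countdown.
; A timeline dips the cylinder and springs it back.
; A flag on the first-person character prevents further presses once one button is used.
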(event EventBeginPlay
  (bind _asbp_first_person_character (Utilities|Casting|CastToBP_FirstPersonCharacter (Game|GetPlayerCharacter 0)))
  (Variables|Default|SetAs%20BP%20First%20Person%20Character _asbp_first_person_character))

(event EventOnInteract
  (params (Character :type BP%20First%20Person%20Character%20Object%20Reference))
  (bind _as_bp_first_person_character (Variables|Default|GetAs%20BP%20First%20Person%20Character))
  (bind _countdown (Variables|/Game/FirstPerson/Blueprints/BP_FirstPersonCharacter.BP_FirstPersonCharacter_C|GetCountdown _as_bp_first_person_character))
  (if (not (Variables|/Game/FirstPerson/Blueprints/BP_FirstPersonCharacter.BP_FirstPersonCharacter_C|GethasPressedButton (Variables|Default|GetAs%20BP%20First%20Person%20Character)))
    (Class|LevelStreamingDynamic|LoadLevelInstancebySoftObjectPtr (Variables|Default|GetRoom%20to%20load) (+ (Transformation|GetWorldLocation (Variables|Default|GetCylinder)) (Variables|Default|GetSpawnRoomPosition)) "0, 0, 0" "" 0 false)
    (Class|IIcone|OnActivate(Message) (Variables|Default|GetPlaneDeLicone) (Variables|Default|GetMaterialDeLiconeQueVousVoulezAfficher) (Variables|Default|GetTimerBonus))
    (Variables|/Game/FirstPerson/Blueprints/BP_FirstPersonCharacter.BP_FirstPersonCharacter_C|SethasPressedButton _as_bp_first_person_character true)
    (Variables|/Game/GP/Widgets/HUD/W_Countdown.W_Countdown_C|Setcountdown _countdown (+ (Variables|/Game/GP/Widgets/HUD/W_Countdown.W_Countdown_C|Getcountdown _countdown) (Variables|Default|GetTimerBonus)))
    (bind _newtrack_0 (Timeline|Timeline Play)
      (:Update
        (Transformation|SetRelativeLocation (Variables|Default|GetCylinder) (Math|Vector|MakeVector 0.0 0.0 (Math|Float|Lerp 0.0 -8.0 _newtrack_0)) false false))
      (:Finished
        (if (not (Variables|Default|GetisPressed))
          (Variables|Default|SetisPressed true)
          (Timeline|Timeline ReverseFromEnd))))))

(fn ConstructionScript)

(fn IsInteractible
  (return true))