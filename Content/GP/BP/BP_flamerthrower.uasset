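; Flamethrower turret hazard whose head sweeps in yaw and reports anything entering its trigger box.
; A timeline started on BeginPlay scales its Zrot track by ValRotation to set TurretHead's relative rotation, using the AtDestination flag to alternate forward and reverse playback indefinitely.
; Box overlap only prints "Dead" as a placeholder kill, with no filter on the overlapping actor and an unconnected DestroyActor.
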(event OnComponentBeginOverlap(Box)
  (params (OverlappedComponent :type Primitive%20Component%20Object%20Reference) (OtherActor :type Actor%20Object%20Reference) (OtherComp :type Primitive%20Component%20Object%20Reference) (OtherBodyIndex :type Integer) (bFromSweep :type Boolean) (SweepResult :type Hit%20Result%20Structure%20%28by%20ref%29))
  (Development|PrintString "Dead"))

(event EventBeginPlay
  (bind _zrot (Timeline|RotationOverTime Play)
    (:Update
      (Transformation|SetRelativeRotation (Variables|Default|GetturretHead) (Math|Rotator|MakeRotator 0.0 0.0 (* _zrot (Variables|Default|GetVal%20rotation))) false false))
    (:Finished
      (if (Variables|Default|GetAtDestination?)
        (Variables|Default|SetAtDestination? false)
        (Timeline|RotationOverTime ReverseFromEnd)
        (else
          (Variables|Default|SetAtDestination? true)
          (Timeline|RotationOverTime PlayFromStart))))))

(fn ConstructionScript)