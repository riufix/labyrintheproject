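; BP_tesla is a timed Tesla trap that freezes the first-person player inside its box while active.
; A looping Delay and FlipFlop toggle IsActive every TimeRemaining seconds.
; Box overlaps track the player, and Tick zeroes walk speed while inside and active, otherwise restoring the cached speed.
; Each toggle also sets the Flash visibility on a BL_Lightning found by class, hiding it when active despite the graph comment stating the opposite.
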(event OnComponentEndOverlap(Box)
  (params (OverlappedComponent :type Primitive%20Component%20Object%20Reference) (OtherActor :type Actor%20Object%20Reference) (OtherComp :type Primitive%20Component%20Object%20Reference) (OtherBodyIndex :type Integer))
  (bind _first_person_chara (Variables|Default|GetFirst%20Person%20Chara))
  ;[1 1 1] outofdeathBox
  (if (== OtherActor _first_person_chara)
    (Variables|Default|SetisIn? false)
    (Variables|/Script/Engine.CharacterMovementComponent|SetMaxWalkSpeed (Variables|/Script/Engine.Character|GetCharacterMovement _first_person_chara) (Variables|Default|GetWalk%20speed))))

(event OnComponentBeginOverlap(Box)
  (params (OverlappedComponent :type Primitive%20Component%20Object%20Reference) (OtherActor :type Actor%20Object%20Reference) (OtherComp :type Primitive%20Component%20Object%20Reference) (OtherBodyIndex :type Integer) (bFromSweep :type Boolean) (SweepResult :type Hit%20Result%20Structure%20%28by%20ref%29))
  ;[1 1 1] insideDeathBox
  (if (== OtherActor (Variables|Default|GetFirst%20Person%20Chara))
    (Variables|Default|SetisIn? true)))

(event Custom|Hide%20particle%20toggle
  ;[1 1 1] Lightning hidden when is not active
  (bind _returnvalue (Actor|GetActorOfClass "/Game/GA/FX/FLASH/BL_Lightning.BL_Lightning_C"))
  (if (Variables|Default|GetisActive?)
    (Rendering|SetVisibility (Variables|/Game/GA/FX/FLASH/BL_Lightning.BL_Lightning_C|Getflash _returnvalue) false false)
    (else
      (Rendering|SetVisibility (Variables|/Game/GA/FX/FLASH/BL_Lightning.BL_Lightning_C|Getflash _returnvalue) true false))))

(event EventBeginPlay
  ;[1 1 1] Activation countdown
  (bind _asbp_first_person_character (Utilities|Casting|CastToBP_FirstPersonCharacter (Game|GetPlayerCharacter 0)))
  (bind _output_get (Variables|Default|SetFirst%20Person%20Chara _asbp_first_person_character))
  (Variables|Default|SetWalk%20speed (Variables|/Script/Engine.CharacterMovementComponent|GetMaxWalkSpeed (Variables|/Script/Engine.Character|GetCharacterMovement _output_get)))
  (Utilities|FlowControl|Delay (Variables|Default|GettimeRemaining) :!label _label)
  (Utilities|FlowControl|FlipFlop
    (:A
      (Variables|Default|SetisActive? true)
      (CallFunction|HideParticleToggle)
      (goto _label))
    (:B
      (Variables|Default|SetisActive? false)
      (CallFunction|HideParticleToggle)
      (goto _label))))

(event EventTick
  (params (DeltaSeconds :type Float%20%28single-precision%29))
  (bind _first_person_chara (Variables|Default|GetFirst%20Person%20Chara))
  (bind _charactermovement (Variables|/Script/Engine.Character|GetCharacterMovement _first_person_chara))
  (if (Variables|Default|GetisIn?)
    (if (Variables|Default|GetisActive?)
      (Variables|/Script/Engine.CharacterMovementComponent|SetMaxWalkSpeed _charactermovement 0.0)
      (else
        (Variables|/Script/Engine.CharacterMovementComponent|SetMaxWalkSpeed _charactermovement (Variables|Default|GetWalk%20speed))))))

(fn ConstructionScript)