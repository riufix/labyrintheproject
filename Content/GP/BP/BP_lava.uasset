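; BP_lava is a lava hazard that kills the first-person player on contact.
; BeginPlay caches the player character and the first-person game mode.
; When that character overlaps the Box, ShowDamage disables movement, shows the game mode's damage HUD and plays a burn sound.
; After a one-second delay the HUD is hidden and the character's CEDie event is called.
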(event OnComponentBeginOverlap(Box)
  (params (OverlappedComponent :type Primitive%20Component%20Object%20Reference) (OtherActor :type Actor%20Object%20Reference) (OtherComp :type Primitive%20Component%20Object%20Reference) (OtherBodyIndex :type Integer) (bFromSweep :type Boolean) (SweepResult :type Hit%20Result%20Structure%20%28by%20ref%29))
  (if (== OtherActor (Variables|Default|GetAs%20BP%20First%20Person%20Character))
    (CallFunction|ShowDamage)
    (Utilities|FlowControl|Delay 1.0)
    (Variables|/Script/UMG.Widget|SetVisibility (Variables|/Game/FirstPerson/Blueprints/BP_FirstPersonGameMode.BP_FirstPersonGameMode_C|GetDamage%20HUD (Variables|Default|GetGame%20mode)) "Hidden")
    (Default|CEDie (Variables|Default|GetAs%20BP%20First%20Person%20Character))))

(event EventBeginPlay
  (bind _asbp_first_person_character (Utilities|Casting|CastToBP_FirstPersonCharacter (Game|GetPlayerCharacter 0)))
  (Variables|Default|SetAs%20BP%20First%20Person%20Character _asbp_first_person_character)
  (bind _asbp_first_person_game_mode (Utilities|Casting|CastToBP_FirstPersonGameMode (Game|GetGameMode))
    (:then
      (Variables|Default|SetGame%20mode _asbp_first_person_game_mode))
    (:CastFailed
      (Development|PrintString "cast failed"))))

(fn ConstructionScript)

(fn ShowDamage
  (Pawn|Components|CharacterMovement|DisableMovement (Variables|/Script/Engine.Character|GetCharacterMovement (Variables|Default|GetAs%20BP%20First%20Person%20Character)))
  (Widget|SetVisibility (Variables|/Game/FirstPerson/Blueprints/BP_FirstPersonGameMode.BP_FirstPersonGameMode_C|GetDamage%20HUD (Variables|Default|GetGame%20mode)) "Visible")
  (Audio|PlaySound2D "/Game/SD/lava_burn.lava_burn" 1.0 1.0 0.0 0 0) ; Son trop long
)