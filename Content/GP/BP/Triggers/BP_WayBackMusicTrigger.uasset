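; BP_WayBackMusicTrigger is a box trigger that switches the music to an ambient pad the first time the player character overlaps it.
; It caches BP_GameInstance at BeginPlay, then on overlap unpauses that instance's Music component and fades it out while fading in a newly spawned 2D AmbientPad sound.
; A DoOnce keeps the crossfade from repeating.
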(event OnComponentBeginOverlap(Box)
  (params (OverlappedComponent :type Primitive%20Component%20Object%20Reference) (OtherActor :type Actor%20Object%20Reference) (OtherComp :type Primitive%20Component%20Object%20Reference) (OtherBodyIndex :type Integer) (bFromSweep :type Boolean) (SweepResult :type Hit%20Result%20Structure%20%28by%20ref%29))
  (bind _as_bp_game_instance (Variables|Default|GetAs%20BP%20Game%20Instance))
  (bind _music (Variables|/Game/FirstPerson/Blueprints/BP_GameInstance.BP_GameInstance_C|GetMusic _as_bp_game_instance))
  (if (== OtherActor (Game|GetPlayerCharacter 0))
    (Utilities|FlowControl|DoOnce false
      (:Completed
        (Class|AudioComponent|SetPaused _music false)
        (Audio|Components|Audio|FadeOut _music 0.3 0.0 "Linear" :!class /Script/Engine.AudioComponent)
        (bind _returnvalue (Audio|SpawnSound2D "/Game/SD/AmbientPad.AmbientPad" 1.0 1.0 0.0 0))
        (Audio|Components|Audio|FadeIn _returnvalue 0.3 1.0 0.0 "Linear" :!class /Script/Engine.AudioComponent)))))

(event EventBeginPlay
  (bind _asbp_game_instance (Utilities|Casting|CastToBP_GameInstance (Game|GetGameInstance))
    (:then
      (Variables|Default|SetAs%20BP%20Game%20Instance _asbp_game_instance))
    (:CastFailed
      (Development|PrintString "cast to game instance failed"))))

(fn ConstructionScript)