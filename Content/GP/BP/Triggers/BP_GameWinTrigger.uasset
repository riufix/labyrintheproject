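; BP_GameWinTrigger is a trigger actor that runs the game-win ending sequence when overlapped.
; Its collision is disabled at BeginPlay so the menu does not show immediately; this file never re-enables it.
; Any overlap disables the cached first-person character's movement, then shows the win, fade and credits widgets in sequence, separated by delays.
; The credits step switches input to UI only, shows the cursor and plays the credits.
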(event Collision|EventActorBeginOverlap
  (params (OtherActor :type Actor%20Object%20Reference))
  (bind _returnvalue (Game|GetPlayerController 0))
  (Pawn|Components|CharacterMovement|DisableMovement (Variables|/Script/Engine.Character|GetCharacterMovement (Variables|Default|GetAs%20BP%20First%20Person%20Character)))
  (bind _returnvalue_2 (UserInterface|CreateWidget "/Game/GP/Widgets/HUD/W_GameWin.W_GameWin_C"))
  (UserInterface|Viewport|AddtoViewport _returnvalue_2 0)
  (Utilities|FlowControl|Delay 2.0)
  (bind _returnvalue_3 (UserInterface|CreateWidget "/Game/GP/Widgets/Menus/W_FadeToNextScene.W_FadeToNextScene_C"))
  (UserInterface|Viewport|AddtoViewport _returnvalue_3 0)
  (Default|PlayFade _returnvalue_3)
  (Utilities|FlowControl|Delay 1.5)
  (bind _returnvalue_4 (UserInterface|CreateWidget "/Game/GP/Widgets/Menus/W_Credits.W_Credits_C"))
  (UserInterface|Viewport|AddtoViewport _returnvalue_4 0)
  (Input|SetInputModeUIOnly _returnvalue 0 "DoNotLock" false)
  (Variables|/Script/Engine.PlayerController|SetbShowMouseCursor _returnvalue true)
  (Default|PlayCredits _returnvalue_4))

(event EventBeginPlay
  ;[1 1 1] Désactive la collision pour pas afficher le menu dès le début
  (Collision|SetActorEnableCollision false)
  (bind _asbp_first_person_character (Utilities|Casting|CastToBP_FirstPersonCharacter (Game|GetPlayerCharacter 0)))
  (Variables|Default|SetAs%20BP%20First%20Person%20Character _asbp_first_person_character))

(fn ConstructionScript)