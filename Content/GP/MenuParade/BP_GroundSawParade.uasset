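; BP_GroundSawParade is a saw hazard on a rotating arm that kills the first-person player character on hit.
; After a TimeToStart delay triggered from Tick, the 180Movement timeline drives the arm's pitch between zero and AngleToOsciliate through its MechanicalMovement track.
; The saw's hit event calls CEDie on the character cached at BeginPlay.
; The arm's DefaultLocation is stored but not used.
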(event OnComponentHit(Saw)
  (params (HitComponent :type Primitive%20Component%20Object%20Reference) (OtherActor :type Actor%20Object%20Reference) (OtherComp :type Primitive%20Component%20Object%20Reference) (NormalImpulse :type Vector :default "0, 0, 0") (Hit :type Hit%20Result%20Structure%20%28by%20ref%29))
  (bind _first_person_chara (Variables|Default|GetFirst%20Person%20Chara))
  ;[1 1 1] Death
  (if (== OtherActor _first_person_chara)
    (Default|CEDie _first_person_chara)))

(event EventBeginPlay
  (bind _asbp_first_person_character (Utilities|Casting|CastToBP_FirstPersonCharacter (Game|GetPlayerCharacter 0)))
  (Variables|Default|SetFirst%20Person%20Chara _asbp_first_person_character))

(event EventTick
  (params (DeltaSeconds :type Float%20%28single-precision%29))
  (Utilities|FlowControl|Delay (Variables|Default|GetTime%20To%20Start))
  (Variables|Default|SetDefaultLocation (Variables|/Script/Engine.SceneComponent|GetRelativeLocation (Variables|Default|Getarm)))
  (bind _mechanical_movement (Timeline|180%20movement Play)
    (:Update
      (Transformation|SetRelativeRotation (Variables|Default|Getarm) (Math|Rotator|MakeRotator 0.0 (Math|Float|Lerp 0.0 (Variables|Default|GetAngle%20To%20Osciliate) _mechanical_movement) 0.0) false false))))

(fn ConstructionScript)